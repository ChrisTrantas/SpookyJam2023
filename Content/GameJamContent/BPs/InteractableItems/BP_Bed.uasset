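; Bed interactable that lets the day advance once it is late enough to sleep.
; On BeginPlay it binds to the DayNightCycle hour update, which sets CanSleep from 19:00 onward and swaps the inspectable object's description to match.
; TrySleepBed increments the day when sleeping is allowed and prints a message either way; its caller is outside this Blueprint.
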(event Custom|HandleHourUpdated
  (params (Hour :type Integer))
  (CallFunction|UpdateBed Hour))

(event EventBeginPlay
  (|CallParentFunction)
  (EventDispatchers|BindEventtoHourUpdated (Variables|Default|GetDayNightCycle) (delegate Custom|HandleHourUpdated)))

(event Collision|EventActorBeginOverlap
  (params (OtherActor :type Actor%20Object%20Reference))
  (|CallParentFunction OtherActor) ; This node is disabled and will not be called.\nDrag off pins to build functionality.
)

(event EventTick
  (params (DeltaSeconds :type Float%20%28single-precision%29))
  (|CallParentFunction DeltaSeconds) ; This node is disabled and will not be called.\nDrag off pins to build functionality.
)

(fn ConstructionScript
  (|CallParentFunction))

(fn UpdateBed
  (params (Hour :type Integer))
  (bind _output_get (Variables|Default|SetCanSleep (>= Hour 19)))
  (if _output_get
    (Variables|/Game/GameJamContent/BPs/InteractableItems/BP_InspectableObject.BP_InspectableObject_C|SetItemDisplayDescription (Variables|Default|GetBP_InspectableObject) "Time to sleep.")
    (else
      (Variables|/Game/GameJamContent/BPs/InteractableItems/BP_InspectableObject.BP_InspectableObject_C|SetItemDisplayDescription (Variables|Default|GetBP_InspectableObject) "It's not time to sleep yet."))))

(fn TrySleepBed
  (if (Variables|Default|GetCanSleep)
    (Default|IncrementDay (Variables|Default|GetDayNightCycle))
    (Development|PrintString "Goodmorning")
    (else
      (Development|PrintString "Can't Sleep Yet"))))