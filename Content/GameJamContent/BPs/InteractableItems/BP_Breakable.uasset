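; BP_Breakable is a component that makes its owning actor breakable, replacing it with spawned actors when broken.
; HandleBreak spawns each class in SpawnedActors at a random-direction offset from the owner, scaled by SpawnDistanceVariance, with random rotation.
; Spawning adjusts for collisions but always succeeds, then the owner is destroyed.
; The file contains no trigger for the break, and BeginPlay and Tick are unused.
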(event EventBeginPlay)

(event EventTick
  (params (DeltaSeconds :type Float%20%28single-precision%29)))

(fn HandleBreak
  (for _array_element (Variables|Default|GetSpawnedActors)
    (Game|SpawnActorfromClass _array_element (Math|Transform|MakeTransform (+ (Transformation|GetActorLocation (Components|GetOwner)) (* (Math|Random|RandomUnitVector) (Variables|Default|GetSpawnDistanceVariance))) (Math|Random|RandomRotator false)) "AdjustIfPossibleButAlwaysSpawn" "MultiplyWithRoot" 0 0))
  (Actor|DestroyActor (Components|GetOwner)))