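; Interactable fireplace that burns added objects, each stored as a heat value and remaining burn time.
; Every Tick it counts down burn times, removes spent items and sums the rest into a heat level.
; A differing total fires FireplaceHeatLevelChanged, and threshold lookup picks the description text shown through its inspectable object.
; Debug prints report additions, heat and an empty fireplace.
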(event EventTick
  (params (DeltaSeconds :type Float%20%28single-precision%29))
  (CallFunction|UpdateBurningItems DeltaSeconds)
  (CallFunction|ClearFinishedItems)
  (bind _fireplaceheat (CallFunction|GetFireplaceHeatLevel))
  (CallFunction|UpdateDisplayedText _fireplaceheat))

(fn ConstructionScript
  (|CallParentFunction))

(fn AddObjecttoBurn
  (params (AddedHeatValue :type Integer) (ObjectBurnDuration :type Float%20%28double-precision%29))
  (Development|PrintString (Utilities|String|ToString(Text) (Utilities|Text|FormatText "Adding Object with heat:{heat} duration:{duration}" AddedHeatValue ObjectBurnDuration)))
  (Utilities|Array|Add (Variables|Default|GetBurningItems) (Utilities|Struct|MakeS_BurningItem AddedHeatValue ObjectBurnDuration)))

(fn GetFireplaceHeatLevel
  (for _array_element (Variables|Default|GetBurningItems)
    (LocalVariables|SetTempHeat (+ (LocalVariables|GetTempHeat) (.HeatValue (Utilities|Struct|BreakS_BurningItem _array_element)))))
  (if (!= (LocalVariables|GetTempHeat) (Variables|Default|GetFireplaceHeatLevel))
    (Default|CallFireplaceHeatLevelChanged (LocalVariables|GetTempHeat))
    (Development|PrintString (Utilities|String|BuildString(Integer) "Fireplace Heat: " "" (LocalVariables|GetTempHeat)) true true "(R=0.000000,G=0.660000,B=1.000000,A=1.000000)" 2.0 "FireplaceStatus")
    (return (LocalVariables|GetTempHeat))))

(fn UpdateBurningItems
  (params (DeltaTime :type Float%20%28double-precision%29))
  (if (Utilities|Array|IsNotEmpty (Variables|Default|GetBurningItems)) ; Are there items to burn?
    (for _array_element (Variables|Default|GetBurningItems)
      (Utilities|Struct|SetmembersinS_BurningItem (Utilities|Struct|MakeS_BurningItem (.HeatValue (Utilities|Struct|BreakS_BurningItem _array_element)) (- (.BurnTimeRemainingInSeconds (Utilities|Struct|BreakS_BurningItem _array_element)) DeltaTime))) ; Update items
    )
    (else
      (Development|PrintString "Fireplace Empty" true true "(R=0.000000,G=0.660000,B=1.000000,A=1.000000)" 2.0 "FireplaceStatus"))))

(fn ClearFinishedItems
  (for (_array_element _array_index) (Variables|Default|GetBurningItems)
    (if (not (> (.BurnTimeRemainingInSeconds (Utilities|Struct|BreakS_BurningItem _array_element)) 0.0)) ; Is Item still burning?
      (Utilities|Array|RemoveIndex (Variables|Default|GetBurningItems) _array_index) ; Remove Burnt Items
    )))

(fn UpdateDisplayedText
  (params (Heat :type Integer))
  (bind _index (Utilities|FlowControl|ForLoopwithBreak 0 5 :!label _label)
    (:LoopBody
      (if (>= Heat (Utilities|Array|Get(acopy) (LocalVariables|GetHeatThresholds) _index))
        (Variables|/Game/GameJamContent/BPs/InteractableItems/BP_InspectableObject.BP_InspectableObject_C|SetItemDisplayDescription (Variables|Default|GetBP_InspectableObject) (Utilities|Array|Get(acopy) (Variables|Default|GetHeatLevelDescriptions) _index))
        (goto _label Break)))))