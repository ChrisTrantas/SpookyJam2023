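; BP_CabinDoor is a cabin door actor that can be opened, closed or blocked by snow.
; TryOpenDoor toggles the door by snapping its relative rotation between closed and a half turn, or only prints a stuck-noise placeholder when blocked.
; SetDoorBlocked forces the door shut and sets the inspectable object's description to report snow, or clears both block and description without reopening it.
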(event EventBeginPlay)

(event Collision|EventActorBeginOverlap
  (params (OtherActor :type Actor%20Object%20Reference)))

(event EventTick
  (params (DeltaSeconds :type Float%20%28single-precision%29)))

(fn ConstructionScript)

(fn TryOpenDoor
  (if (Variables|Default|GetDoorBlocked)
    (Development|PrintString "Door is Blocked, play door stuck noise")
    (elif (Variables|Default|GetIsDoorOpen)
      (Development|PrintString "Close Door")
      (Variables|Default|SetIsDoorOpen false)
      (Transformation|SetRelativeRotation (Variables|Default|GetDoor) "0, 0, 0" false false)
      (else
        (Development|PrintString "Open Door")
        (Variables|Default|SetIsDoorOpen true)
        (Transformation|SetRelativeRotation (Variables|Default|GetDoor) "0.000000,180.000000,0.000000" false false)))))

(fn SetDoorBlocked
  (params (IsBlocked :type Boolean))
  (if IsBlocked
    (Transformation|SetRelativeRotation (Variables|Default|GetDoor) "0, 0, 0" false false)
    (Variables|Default|SetIsDoorOpen false)
    (Variables|Default|SetDoorBlocked true)
    (Variables|/Game/GameJamContent/BPs/InteractableItems/BP_InspectableObject.BP_InspectableObject_C|SetItemDisplayDescription (Variables|Default|GetBP_InspectableObject) "Blocked by snow.")
    (else
      (Variables|Default|SetDoorBlocked false)
      (Variables|/Game/GameJamContent/BPs/InteractableItems/BP_InspectableObject.BP_InspectableObject_C|SetItemDisplayDescription (Variables|Default|GetBP_InspectableObject) ""))))