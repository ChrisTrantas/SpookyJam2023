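; BP_InteriorVolume is a trigger volume in the heat system that tracks whether the player is inside the cabin.
; Begin and end overlaps on InteriorTriggerVolume respond only to BP_GameJamCharacter and call enter and exit handler functions.
; Those handlers only set the IsPlayerInsideCabin flag, with no heat logic in this graph.
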(event OnComponentBeginOverlap(InteriorTriggerVolume)
  (params (OverlappedComponent :type Primitive%20Component%20Object%20Reference) (OtherActor :type Actor%20Object%20Reference) (OtherComp :type Primitive%20Component%20Object%20Reference) (OtherBodyIndex :type Integer) (bFromSweep :type Boolean) (SweepResult :type Hit%20Result%20Structure%20%28by%20ref%29))
  (if (Class|GameplayStatics|ObjectIsA OtherActor "/Game/GameJamContent/BPs/Player/BP_GameJamCharacter.BP_GameJamCharacter_C")
    (CallFunction|HandlePlayerEnterCabin)))

(event OnComponentEndOverlap(InteriorTriggerVolume)
  (params (OverlappedComponent :type Primitive%20Component%20Object%20Reference) (OtherActor :type Actor%20Object%20Reference) (OtherComp :type Primitive%20Component%20Object%20Reference) (OtherBodyIndex :type Integer))
  (if (Class|GameplayStatics|ObjectIsA OtherActor "/Game/GameJamContent/BPs/Player/BP_GameJamCharacter.BP_GameJamCharacter_C")
    (CallFunction|HandlePlayerExitCabin)))

(fn ConstructionScript)

(fn HandlePlayerEnterCabin
  (Variables|Default|SetIsPlayerInsideCabin true))

(fn HandlePlayerExitCabin
  (Variables|Default|SetIsPlayerInsideCabin false))