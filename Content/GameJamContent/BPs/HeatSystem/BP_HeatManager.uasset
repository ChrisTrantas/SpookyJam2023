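; BP_HeatManager computes the ambient temperature around the player, inside or outside a cabin.
; On BeginPlay it finds the interior volume, cabin door, fireplace and day-night cycle actors in the level.
; Exterior heat is a temperature looked up by hour plus a per-day offset.
; Interior heat adds the fireplace's level to that, plus an insulation bonus only while the door is closed.
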(event EventBeginPlay
  (bind _returnvalue (Actor|GetActorOfClass "/Game/GameJamContent/BPs/HeatSystem/BP_InteriorVolume.BP_InteriorVolume_C"))
  (Variables|Default|SetInteriorVolume _returnvalue)
  (bind _returnvalue_2 (Actor|GetActorOfClass "/Game/GameJamContent/BPs/HeatSystem/BP_CabinDoor.BP_CabinDoor_C"))
  (Variables|Default|SetDoorReference _returnvalue_2)
  (bind _returnvalue_3 (Actor|GetActorOfClass "/Game/GameJamContent/BPs/InteractableItems/BP_Fireplace.BP_Fireplace_C"))
  (Variables|Default|SetFireplaceReference _returnvalue_3)
  (bind _returnvalue_4 (Actor|GetActorOfClass "/Game/GameJamContent/BPs/BP_DayNightCycle.BP_DayNightCycle_C"))
  (Variables|Default|SetDayNightCycleTimeline _returnvalue_4))

(fn CalculateInteriorHeat
  (params (DayIndex :type Integer) (HourNumber :type Integer))
  (bind _currentheat (CallFunction|CalculateExteriorHeat DayIndex HourNumber))
  (LocalVariables|SetCurrentOutdoorHeat _currentheat)
  (if (not (Variables|/Game/GameJamContent/BPs/HeatSystem/BP_CabinDoor.BP_CabinDoor_C|GetIsDoorOpen (Variables|Default|GetDoorReference)))
    (bind _fireplaceheat (Default|GetFireplaceHeatLevel (Variables|Default|GetFireplaceReference)))
    (return (+ _fireplaceheat (Variables|Default|GetFunctioningInteriorBonus) (LocalVariables|GetCurrentOutdoorHeat)))
    (else
      (bind _fireplaceheat_2 (Default|GetFireplaceHeatLevel (Variables|Default|GetFireplaceReference)))
      (return (+ _fireplaceheat_2 (LocalVariables|GetCurrentOutdoorHeat))))))

(fn CalculateExteriorHeat
  (params (DayIndex :type Integer) (HourNumber :type Integer))
  (bind _temperaturebyhour (Variables|Default|GetTemperatureByHour))
  (bind (_value _returnvalue) (Utilities|Map|Find _temperaturebyhour HourNumber))
  (if _returnvalue
    (return (+ (Utilities|Array|Get(acopy) (Variables|Default|GetTemperatureOffsetByDay) DayIndex) _value))
    (else
      (Development|PrintString "ERR; INVALID HOUR" true true "(R=1.000000,G=0.000000,B=0.123857,A=1.000000)"))))

(fn GetCurrentAmbientHeat
  (bind _daynightcycletimeline (Variables|Default|GetDayNightCycleTimeline))
  (bind _solartime (Variables|/Game/GameJamContent/BPs/BP_DayNightCycle.BP_DayNightCycle_C|GetSolarTime _daynightcycletimeline))
  (bind _daycounter (Variables|/Game/GameJamContent/BPs/BP_DayNightCycle.BP_DayNightCycle_C|GetDayCounter _daynightcycletimeline))
  (bind _returnvalue (Math|Float|Truncate _solartime))
  (if (Variables|/Game/GameJamContent/BPs/HeatSystem/BP_InteriorVolume.BP_InteriorVolume_C|GetIsPlayerInsideCabin (Variables|Default|GetInteriorVolume))
    (bind _currentheat (CallFunction|CalculateInteriorHeat _daycounter _returnvalue))
    (return _currentheat)
    (else
      (bind _currentheat_2 (CallFunction|CalculateExteriorHeat _daycounter _returnvalue))
      (return _currentheat_2))))