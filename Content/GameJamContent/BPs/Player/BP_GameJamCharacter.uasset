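; First-person player character for a game jam survival game, handling object inspection, interaction and frostbite.
; Near inspectables, a looping sphere trace updates HUD info and a context cursor chosen by gameplay-tag names.
; Interact traces again to grab, drop, burn held items in fireplaces or break objects with an axe; the door branch only looks up the cabin door.
; A non-looping BeginPlay timer applies ambient heat to frostbite, which can trigger death.
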(event OnComponentBeginOverlap(InteractionTestSphere)
  (params (OverlappedComponent :type Primitive%20Component%20Object%20Reference) (OtherActor :type Actor%20Object%20Reference) (OtherComp :type Primitive%20Component%20Object%20Reference) (OtherBodyIndex :type Integer) (bFromSweep :type Boolean) (SweepResult :type Hit%20Result%20Structure%20%28by%20ref%29))
  (Utilities|IsValid (Actor|GetComponentbyClass OtherActor "/Game/GameJamContent/BPs/InteractableItems/BP_InspectableObject.BP_InspectableObject_C")
    (:Is%20Valid
      (Variables|ObjectInspecting|SetWithinInspectRange true)
      (Utilities|Time|SetTimerbyFunctionName 0 "CheckInspectableVisible" (Variables|ObjectInspecting|GetInspectUpdateFrequency) true)
      (Development|PrintString "In Range of Inspectables" true true "(R=0.000000,G=0.660000,B=1.000000,A=1.000000)" 2.0 "Inspect"))))

(event OnComponentEndOverlap(InteractionTestSphere)
  (params (OverlappedComponent :type Primitive%20Component%20Object%20Reference) (OtherActor :type Actor%20Object%20Reference) (OtherComp :type Primitive%20Component%20Object%20Reference) (OtherBodyIndex :type Integer))
  (if (== 0 (Utilities|Array|Length (Collision|GetOverlappingActors "/Game/GameJamContent/BPs/InteractableItems/BP_InteractableObject.BP_InteractableObject_C" :!class /Script/Engine.Actor)))
    (Variables|ObjectInspecting|SetWithinInspectRange false)
    (Utilities|Time|ClearTimerbyFunctionName 0 "CheckInspectableVisible")
    (Development|PrintString "Out of Range of Inspectables" true true "(R=0.000000,G=0.660000,B=1.000000,A=1.000000)" 2.0 "Inspect")))

(event Input|EnhancedActionEvents|EnhancedInputActionIA_Interact
  (params (ActionValue :type Boolean) (ElapsedSeconds :type Float%20%28double-precision%29) (TriggeredSeconds :type Float%20%28double-precision%29) (InputAction :type Input%20Action%20Object%20Reference :default "/Game/FirstPerson/Input/Actions/IA_Interact.IA_Interact"))
  (:Triggered
    (Interaction|AttemptInteract)))

(event EventBeginPlay
  (|CallParentFunction)
  (Default|CallOnClearInspectionHUD)
  (Default|CallUpdateCursorAction "NewEnumerator0")
  (Utilities|Time|SetTimerbyFunctionName 0 "ManageHeat" 0.2))

(event EventTick
  (params (DeltaSeconds :type Float%20%28single-precision%29)))

(fn ConstructionScript
  (|CallParentFunction))

(fn CheckInspectableVisible
  (bind (_start _end) (Utilities|GetTracePath))
  (bind _outhit (Collision|SphereTraceByChannel _start _end 1e+01 "TraceTypeQuery3" false (Utilities|Array|MakeArray (Variables|ObjectHolding|GetHeldObjectActor)) "None"))
  (if (.bBlockingHit (Collision|BreakHitResult _outhit))
    (Utilities|IsValid (Actor|GetComponentbyClass (.HitActor (Collision|BreakHitResult _outhit)) "/Game/GameJamContent/BPs/InteractableItems/BP_InspectableObject.BP_InspectableObject_C")
      (:Is%20Valid
        (Development|PrintString "Hit Object" true true "(R=0.000000,G=0.660000,B=1.000000,A=1.000000)" 2.0 "InspectRaycast")
        (bind _output_get (LocalVariables|SetHitInspectableObject (Actor|GetComponentbyClass (.HitActor (Collision|BreakHitResult _outhit)) "/Game/GameJamContent/BPs/InteractableItems/BP_InspectableObject.BP_InspectableObject_C")))
        (bind (_displayname _displaydescription _tags) (Default|GetDisplayInfo _output_get))
        (Default|CallUpdateObjectInfo _displayname _displaydescription)
        (if (Variables|ObjectHolding|GetIsHoldingObject)
          (bind _cursortype (CursorControl|DetermineCursorWhileHolding _tags (Variables|/Script/Engine.Actor|GetTags (Variables|ObjectHolding|GetHeldObjectActor))))
          (Default|CallUpdateCursorAction _cursortype)
          (else
            (bind _cursortype_2 (CursorControl|DetermineCursorHandsEmpty _tags))
            (Default|CallUpdateCursorAction _cursortype_2))))
      (:Is%20Not%20Valid
        (Development|PrintString "Invalid Hit" true true "(R=0.000000,G=0.660000,B=1.000000,A=1.000000)" 2.0 "InspectRaycast")
        (Default|CallOnClearInspectionHUD)
        (Default|CallUpdateCursorAction "NewEnumerator0")))
    (else
      (Development|PrintString "No Hits" true true "(R=0.000000,G=0.660000,B=1.000000,A=1.000000)" 2.0 "InspectRaycast")
      (Default|CallOnClearInspectionHUD)
      (Default|CallUpdateCursorAction "NewEnumerator0"))))

(fn AttemptInteract
  (bind (_start _end) (Utilities|GetTracePath))
  (bind (_start_2 _end_2) (Utilities|GetTracePath))
  (if (Variables|ObjectHolding|GetIsHoldingObject)
    (bind (_outhit _returnvalue) (Collision|SphereTraceByChannel _start _end 1e+01 "TraceTypeQuery3" false (Utilities|Array|MakeArray (Variables|ObjectHolding|GetHeldObjectActor)) "None"))
    (bind _output_get (LocalVariables|SetHitResult _outhit))
    (LocalVariables|SetHitActor (.HitActor (Collision|BreakHitResult _output_get)))
    (if _returnvalue
      (if (Utilities|IsActorFireplace (LocalVariables|GetHitActor)) ; Looking at fire?
        (if (Utilities|IsActorBurnable (Variables|ObjectHolding|GetHeldObjectActor)) ; Held object burnable?
          (bind _asbp_fireplace (Utilities|Casting|CastToBP_Fireplace (LocalVariables|GetHitActor)))
          (Interaction|BurnObject (Variables|ObjectHolding|GetHeldObjectActor) _asbp_fireplace)
          (else
            (Development|PrintString "Held Object not Burnable" true true "(R=0.000000,G=0.660000,B=1.000000,A=1.000000)" 2.0 "Interaction")))
        (elif (Utilities|IsActorAxe (Variables|ObjectHolding|GetHeldObjectActor)) ; Held Object is Axe?
          (if (Utilities|IsActorBreakable (LocalVariables|GetHitActor)) ; Looking at Breakable?
            (Interaction|BreakObject (LocalVariables|GetHitActor))
            (else
              (Development|PrintString "Hit Object Not Breakable" true true "(R=0.000000,G=0.660000,B=1.000000,A=1.000000)" 2.0 "Interaction")))))
      (else
        (Interaction|DropObject)))
    (else
      (bind (_outhit_2 _returnvalue_2) (Collision|SphereTraceByChannel _start_2 _end_2 1e+01 "TraceTypeQuery3" false 0 "None"))
      (bind _output_get_2 (LocalVariables|SetHitResult _outhit_2))
      (LocalVariables|SetHitActor (.HitActor (Collision|BreakHitResult _output_get_2)))
      (if _returnvalue_2
        (if (Utilities|IsActorDoor (LocalVariables|GetHitActor))
          (Interaction|TryOpenDoor)
          (elif (Utilities|IsActorGrabbable (LocalVariables|GetHitActor))
            (Interaction|GrabObject (LocalVariables|GetHitResult))
            (else
              (Development|PrintString "Not Grabbable" true true "(R=0.000000,G=0.660000,B=1.000000,A=1.000000)" 2.0 "Interaction"))))
        (else
          (Development|PrintString "Nothing There" true true "(R=0.000000,G=0.660000,B=1.000000,A=1.000000)" 2.0 "Interaction"))))))

(fn DropObject
  (Default|CallUpdateCursorAction "NewEnumerator0")
  (Transformation|DetachFromActor (Variables|ObjectHolding|GetHeldObjectActor) "KeepWorld" "KeepWorld" "KeepWorld")
  (Class|PrimitiveComponent|WakeRigidBody (Actor|GetComponentbyClass (Variables|ObjectHolding|GetHeldObjectActor) "/Script/Engine.PrimitiveComponent") "None")
  (Physics|SetPhysicsLinearVelocity (Actor|GetComponentbyClass (Variables|ObjectHolding|GetHeldObjectActor) "/Script/Engine.PrimitiveComponent") "0, 0, 0" false "None")
  (Physics|SetEnableGravity (Actor|GetComponentbyClass (Variables|ObjectHolding|GetHeldObjectActor) "/Script/Engine.PrimitiveComponent") true)
  (Physics|SetSimulatePhysics (Actor|GetComponentbyClass (Variables|ObjectHolding|GetHeldObjectActor) "/Script/Engine.PrimitiveComponent") true)
  (Development|PrintString "Dropping Held Object" true true "(R=0.000000,G=0.660000,B=1.000000,A=1.000000)" 2.0 "Interaction")
  (Variables|ObjectHolding|SetHeldObjectActor 0)
  (Variables|ObjectHolding|SetIsHoldingObject false))

(fn GrabObject
  (params (HitResult :type Hit%20Result%20Structure))
  (bind _hitactor (Collision|BreakHitResult HitResult))
  (Default|CallUpdateCursorAction "NewEnumerator0")
  (Development|PrintString "Attempting Grab" true true "(R=0.000000,G=0.660000,B=1.000000,A=1.000000)" 2.0 "Interaction")
  (Transformation|SetWorldLocation (Variables|/Script/Engine.Actor|GetRootComponent _hitactor) (Transformation|GetWorldLocation (Variables|Default|GetHeldObjectSlot)) false true)
  (Transformation|AttachComponentToComponent _hitactor (Variables|Default|GetHeldObjectSlot) "None" "SnapToTarget" "SnapToTarget" "KeepWorld" true)
  (Variables|ObjectHolding|SetHeldObjectActor (.HitActor (Collision|BreakHitResult HitResult)))
  (Variables|ObjectHolding|SetIsHoldingObject true))

(fn BurnObject
  (params (ObjectToBurn :type Actor%20Object%20Reference) (FireplaceActor :type BP%20Fireplace%20Object%20Reference))
  (bind _returnvalue (Actor|GetComponentbyClass ObjectToBurn "/Game/GameJamContent/BPs/InteractableItems/BP_Burnable.BP_Burnable_C"))
  (Utilities|IsValid _returnvalue
    (:Is%20Valid
      (bind (_addedheatvalue _burnduration) (Default|GetBurnData _returnvalue))
      (Default|AddObjecttoBurn FireplaceActor _addedheatvalue _burnduration)
      (Default|BurnObject _returnvalue)
      (Development|PrintString "Object Burned" true true "(R=0.000000,G=0.660000,B=1.000000,A=1.000000)" 2.0 "Interaction")
      (Variables|ObjectHolding|SetHeldObjectActor 0)
      (Variables|ObjectHolding|SetIsHoldingObject false)
      (Default|CallUpdateCursorAction "NewEnumerator0"))
    (:Is%20Not%20Valid
      (Development|PrintString "Failed to find Burnable Component" true true "(R=0.000000,G=0.660000,B=1.000000,A=1.000000)" 2.0 "Interaction"))))

(fn BreakObject
  (params (Object%20to%20Break :type Actor%20Object%20Reference))
  (bind _returnvalue (Actor|GetComponentbyClass Object%20to%20Break "/Game/GameJamContent/BPs/InteractableItems/BP_Breakable.BP_Breakable_C"))
  (Utilities|IsValid _returnvalue
    (:Is%20Valid
      (Default|CallUpdateCursorAction "NewEnumerator0")
      (Default|HandleBreak _returnvalue)
      (Development|PrintString "Object Broken" true true "(R=0.000000,G=0.660000,B=1.000000,A=1.000000)" 2.0 "Interaction"))
    (:Is%20Not%20Valid
      (Development|PrintString "Failed to Find Breakable Component" true true "(R=0.000000,G=0.660000,B=1.000000,A=1.000000)" 2.0 "Interaction"))))

(fn DetermineCursorWhileHolding
  (params (HitActorTags :type Array%20of%20Names) (HeldActorTags :type Array%20of%20Names))
  (if (Utilities|Array|ContainsItem HitActorTags (GameplayTags|GetTagName (GameplayTags|MakeLiteralGameplayTag "(TagName=\"Interactable.Fireplace\")"))) ; Am I looking at the fire?
    (if (Utilities|Array|ContainsItem HeldActorTags (GameplayTags|GetTagName (GameplayTags|MakeLiteralGameplayTag "(TagName=\"Interactable.Burnable\")"))) ; Holding Something Burnable?
      (return "NewEnumerator1")
      (else
        (return "NewEnumerator0")))
    (elif (Utilities|Array|ContainsItem HitActorTags (GameplayTags|GetTagName (GameplayTags|MakeLiteralGameplayTag "(TagName=\"Interactable.Breakable\")"))) ; Am I looking at something breakable?
      (if (Utilities|Array|ContainsItem HeldActorTags (GameplayTags|GetTagName (GameplayTags|MakeLiteralGameplayTag "(TagName=\"Interactable.Axe\")"))) ; Am I holding the Axe?
        (return "NewEnumerator2")
        (else
          (return "NewEnumerator0")))
      (else
        (return "NewEnumerator0")))))

(fn DetermineCursorHandsEmpty
  (params (HitActorTags :type Array%20of%20Names))
  (if (Utilities|Array|ContainsItem HitActorTags (GameplayTags|GetTagName (GameplayTags|MakeLiteralGameplayTag "(TagName=\"Interactable.Grabbable\")"))) ; Can I grab what I'm looking at?
    (return "NewEnumerator3")
    (else
      (return "NewEnumerator0"))))

(fn ManageFrostbite
  (bind _output_get (Variables|Default|SetCurrentFrostbiteLevel (- (Variables|Default|GetCurrentFrostbiteLevel) (Math|Conversions|ToFloat(Integer) (Variables|Default|GetCurrentPlayerHeat)))))
  (Default|CallUpdatePlayerFrostbite (/ _output_get (Variables|Default|GetMaxFrostbiteLevel)))
  (if (>= (Variables|Default|GetCurrentFrostbiteLevel) (Variables|Default|GetMaxFrostbiteLevel))
    (Default|CallPlayerDied)
    (Development|PrintString "Player is Dead" true true "(R=0.967075,G=0.000000,B=1.000000,A=1.000000)")))

(fn ManageHeat
  (bind _currentambientheat (Default|GetCurrentAmbientHeat (Variables|Default|GetBP_HeatManager)))
  (Variables|Default|SetCurrentPlayerHeat _currentambientheat)
  (CallFunction|ManageFrostbite))

(fn TryOpenDoor
  (Actor|GetActorOfClass "/Game/GameJamContent/BPs/HeatSystem/BP_CabinDoor.BP_CabinDoor_C"))