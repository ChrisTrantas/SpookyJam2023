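; BP_JamGameMode is the game jam's game mode Blueprint that sets up the player's on-screen UI.
; On BeginPlay it creates frostbite indicator, heat meter, HUD and clock widgets for player controller 0 and adds each to the viewport.
; The construction script is empty and the file holds no other game rules.
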(event EventBeginPlay
  (bind _returnvalue (Game|GetPlayerController 0))
  (bind _returnvalue_2 (UserInterface|CreateWidget "/Game/GameJamContent/BPs/Player/UI_FrostbiteIndicator.UI_FrostbiteIndicator_C" (Game|GetPlayerController 0)))
  (UserInterface|Viewport|AddtoViewport _returnvalue_2 0)
  (bind _returnvalue_3 (UserInterface|CreateWidget "/Game/GameJamContent/BPs/Player/UI_HeatMeter.UI_HeatMeter_C" (Game|GetPlayerController 0)))
  (UserInterface|Viewport|AddtoViewport _returnvalue_3 0)
  (bind _returnvalue_4 (UserInterface|CreateWidget "/Game/GameJamContent/BPs/InteractableItems/UI_HUD.UI_HUD_C" _returnvalue))
  (UserInterface|Viewport|AddtoViewport _returnvalue_4 0)
  (bind _returnvalue_5 (UserInterface|CreateWidget "/Game/GameJamContent/BPs/Player/UI_Clock.UI_Clock_C" _returnvalue))
  (UserInterface|Viewport|AddtoViewport _returnvalue_5 0))

(fn ConstructionScript)